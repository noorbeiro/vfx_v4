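; BP_particles is an area-effect volume that reveals a Niagara particle effect when a Character overlaps its box.
; On BeginPlay it hides the box and Niagara components and plays a 2D sound.
; Both begin and end overlap set them visible, so the effect stays shown after the Character leaves.
; The construction script sizes the box from Size, while its Niagara vector write targets an unset variable name.
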(event `self.ReceiveBeginPlay`
  (`self.isvisible` false)
  (`GameplayStatics.PlaySound2D` "/Engine/EditorSounds/GamePreview/PossessPlayer.PossessPlayer" 1.0 1.0 0.0 null null))

(event `isvisible`
  (params (`visible?` :type Boolean))
  (`SceneComponent.SetVisibility` (`self.Box`) `visible?` false)
  (`SceneComponent.SetVisibility` (`self.Niagara`) `visible?` false))

(event `self.Box.OnComponentBeginOverlap`
  (params (OverlappedComponent :type "PrimitiveComponent Object Reference") (OtherActor :type "Actor Object Reference") (OtherComp :type "PrimitiveComponent Object Reference") (OtherBodyIndex :type Integer) (bFromSweep :type Boolean) (SweepResult :type "HitResult Structure (by ref)"))
  (cast `Character` OtherActor)
  (`self.isvisible` true))

(event `self.Box.OnComponentEndOverlap`
  (params (OverlappedComponent :type "PrimitiveComponent Object Reference") (OtherActor :type "Actor Object Reference") (OtherComp :type "PrimitiveComponent Object Reference") (OtherBodyIndex :type Integer))
  (cast `Character` OtherActor)
  (`self.isvisible` true))

(fn `UserConstructionScript`
  (`BoxComponent.SetBoxExtent` (`self.Box`) (`self.size`) true)
  (`NiagaraComponent.SetVariableVec3` (`self.Niagara`) "None" (0.0 0.0 0.0)))