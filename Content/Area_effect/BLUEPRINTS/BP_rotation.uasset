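; BP_rotation is an area-effect actor with a rotating movement component and a Plane that appear when a Character touches its Box.
; BeginPlay hides the rotating component's updated primitive and the Plane, then plays the 2D Enter_Simulate sound.
; A shared visibility event toggles both without propagating to children.
; Both begin and end overlap set visibility to true, so they stay shown after the Character leaves.
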(event `self.ReceiveBeginPlay`
  (`self.visibility` false)
  (`GameplayStatics.PlaySound2D` "/Engine/VREditor/Sounds/UI/Enter_Simulate.Enter_Simulate" 1.0 1.0 0.0 null null))

(event `visibility`
  (params (`visible?` :type Boolean))
  (`SceneComponent.SetVisibility` (`MovementComponent.UpdatedPrimitive` (`self.RotatingMovement`)) `visible?` false)
  (`SceneComponent.SetVisibility` (`self.Plane`) `visible?` false))

(event `self.Box.OnComponentBeginOverlap`
  (params (OverlappedComponent :type "PrimitiveComponent Object Reference") (OtherActor :type "Actor Object Reference") (OtherComp :type "PrimitiveComponent Object Reference") (OtherBodyIndex :type Integer) (bFromSweep :type Boolean) (SweepResult :type "HitResult Structure (by ref)"))
  (cast `Character` OtherActor)
  (`self.visibility` true))

(event `self.Box.OnComponentEndOverlap`
  (params (OverlappedComponent :type "PrimitiveComponent Object Reference") (OtherActor :type "Actor Object Reference") (OtherComp :type "PrimitiveComponent Object Reference") (OtherBodyIndex :type Integer))
  (cast `Character` OtherActor)
  (`self.visibility` true))

(fn `UserConstructionScript`)